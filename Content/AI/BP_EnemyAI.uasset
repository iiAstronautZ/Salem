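; BP_EnemyAI is an enemy actor that is destroyed by a single projectile overlap and tracks itself in the game mode's enemy count.
; On BeginPlay it caches the BaseGameMode and increments EnemyRemaining.
; A capsule overlap with either BP_FirstPersonProjectile or TheWitchTrialsProjectile decrements the count, calls CheckEnemyLeft and destroys the enemy.
; The graphs contain no movement or behavior logic.
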(event OnComponentBeginOverlap(CapsuleComponent)
  (params (OverlappedComponent :type Primitive%20Component%20Object%20Reference) (OtherActor :type Actor%20Object%20Reference) (OtherComp :type Primitive%20Component%20Object%20Reference) (OtherBodyIndex :type Integer) (bFromSweep :type Boolean) (SweepResult :type Hit%20Result%20Structure%20%28by%20ref%29))
  (bind _base_game_mode_ref (Variables|Default|GetBase%20Game%20Mode%20Ref))
  (Utilities|Casting|CastToBP_FirstPersonProjectile OtherActor
    (:then
      _)
    (:CastFailed
      (Utilities|Casting|CastToTheWitchTrialsProjectile OtherActor)))
  (Math|Integer|DecrementInt (Variables|/Game/Blueprints/BaseGameMode.BaseGameMode_C|GetEnemyRemaining _base_game_mode_ref)
    (:%20%20
      (Default|CheckEnemyLeft _base_game_mode_ref)
      (Actor|DestroyActor))))

(event EventBeginPlay
  (bind _asbase_game_mode (Utilities|Casting|CastToBaseGameMode (Game|GetGameMode)))
  (Variables|Default|SetBase%20Game%20Mode%20Ref _asbase_game_mode)
  (Math|Integer|IncrementInt (Variables|/Game/Blueprints/BaseGameMode.BaseGameMode_C|GetEnemyRemaining _asbase_game_mode)))

(event Collision|EventActorBeginOverlap
  (params (OtherActor :type Actor%20Object%20Reference)))

(event EventTick
  (params (DeltaSeconds :type Float%20%28single-precision%29)))

(fn ConstructionScript)