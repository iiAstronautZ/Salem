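; Game mode that runs escalating waves of BP_EnemyAI enemies.
; BeginPlay caches the level's BP_EnemySpawn actors after a short delay.
; CheckEnemyLeft fires the SpawnNextWave dispatcher when EnemyRemaining is zero, prints countdown messages, waits, then spawns the wave at random cached points, slightly raised.
; Each wave raises both the enemy count and its increment, so growth accelerates; EnemyRemaining is only read here.
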(event Custom|CheckEnemyLeft
  (bind _enemyspawnsinlevel (Variables|Default|GetEnemySpawnsInLevel))
  (bind _maxint (Variables|Default|GetMaxInt))
  (bind _returnvalue (Math|Random|RandomInteger _maxint))
  (bind _output (Utilities|Array|Get(acopy) _enemyspawnsinlevel _returnvalue))
  (bind _returnvalue_2 (Transformation|GetActorTransform _output))
  (if (== (Variables|Default|GetEnemyRemaining) 0)
    (Default|CallSpawnNextWave)
    (Development|PrintString "Next Wave Start")
    (Development|PrintString "Next Wave Countdown")
    (Utilities|FlowControl|Delay 5.0)
    (Development|PrintString "Next Wave Start")
    (bind _result (Math|Integer|IncrementInt (Variables|Default|GetWave))
      (:%20%20
        (Variables|Default|SetWave _result)
        (for _index (range 0 (- (Variables|Default|GetEnemySpawned) 1))
          (Game|SpawnActorfromClass "/Game/AI/BP_EnemyAI.BP_EnemyAI_C" (Math|Transform|MakeTransform (Math|Vector|MakeVector (.x (.location _returnvalue_2)) (.y (.location _returnvalue_2)) (+ (.z (.location _returnvalue_2)) 5e+01)) (.rotation _returnvalue_2) (.scale _returnvalue_2)) "Undefined" 0 0))
        (Math|Integer|IncrementInt (Variables|Default|GetEnemyIncrement)
          (:%20%20
            (Variables|Default|SetEnemySpawned (+ (Variables|Default|GetEnemySpawned) (Variables|Default|GetEnemyIncrement)))))))))

(event Custom|SpawnNextWave_Event)

(event EventBeginPlay
  (Utilities|FlowControl|Delay 1.0)
  (bind _outactors (Actor|GetAllActorsOfClass "/Game/AI/BP_EnemySpawn.BP_EnemySpawn_C"))
  (bind _output_get (Variables|Default|SetEnemySpawnsInLevel _outactors))
  (Variables|Default|SetMaxInt (+ (Utilities|Array|LastIndex _output_get) 1)))

(fn ConstructionScript)